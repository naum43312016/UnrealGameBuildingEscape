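; An openable door actor that swings open and closed when the OpenDoor component's OnOpen and OnClose events fire.
; It caches its starting rotation at BeginPlay, then the DoorSwing timeline adds its DoorAngle yaw to that rotation each update.
; A timeline event track plays the Doorlock sound at the door's location, and closing reverses the same timeline.
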(event OnClose(OpenDoor)
  (bind _door_angle (Timeline|Door%20Swing Reverse)
    (:Update
      (Transformation|SetActorRotation (Math|Rotator|CombineRotators (Math|Rotator|MakeRotator 0.0 0.0 _door_angle) (Variables|Default|GetInitRotation))))
    (:Audio%20Timing
      (Audio|PlaySoundatLocation "/Game/Audio/door-lock.door-lock" (Transformation|GetActorLocation) "0, 0, 0" 1.0 1.0 0.0 0 0 0))))

(event OnOpen(OpenDoor)
  (bind _door_angle (Timeline|Door%20Swing Play)
    (:Update
      (Transformation|SetActorRotation (Math|Rotator|CombineRotators (Math|Rotator|MakeRotator 0.0 0.0 _door_angle) (Variables|Default|GetInitRotation))))
    (:Audio%20Timing
      (Audio|PlaySoundatLocation "/Game/Audio/door-lock.door-lock" (Transformation|GetActorLocation) "0, 0, 0" 1.0 1.0 0.0 0 0 0))))

(event EventBeginPlay
  (Variables|Default|SetInitRotation (Transformation|GetActorRotation)))

(fn ConstructionScript)